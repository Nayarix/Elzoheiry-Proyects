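; BP_Plataform is a platform prop that rises 350 units vertically shortly after play begins.
; StartFloting records the starting Z, then plays a Timeline whose alpha lerps the actor's height while keeping X and Y.
; StopFloting reverses that Timeline to bring it back down, and the Timeline's Finished output calls OnFloatTimelineFinished.
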(event `self.ReceiveBeginPlay`
  (`KismetSystemLibrary.Delay` 0.5)
  (`self.StartFloting`))

(event `StartFloting`
  (bind (_returnvalue_x _returnvalue_y _returnvalue_z) (`KismetMathLibrary.BreakVector` (`self.K2_GetActorLocation`)))
  (bind (_returnvalue_x_2 _returnvalue_y_2) (`KismetMathLibrary.BreakVector` (`self.K2_GetActorLocation`)))
  (bind _initial_value_z (`self.Initial Value Z`))
  (set `self.Initial Value Z` _returnvalue_z)
  (bind (_direction _alphaz) (`Timeline|Timeline` :!label _label)
    (:`Update`
      (`self.K2_SetActorLocation` (`KismetMathLibrary.MakeVector` _returnvalue_x_2 _returnvalue_y_2 (`KismetMathLibrary.Lerp` _initial_value_z (+ _initial_value_z 350.0) _alphaz))))
    (:`Finished`
      (`self.OnFloatTimelineFinished`))))

(event `StopFloting`
  (goto _label :!via `Reverse`))

(fn `UserConstructionScript`)