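; Base Blueprint for area-of-effect blasts that adds visual and audio feedback to the inherited Trigger behavior.
; Trigger calls the parent implementation, then spawns the blast particle effect on the root component and plays the blast sound at the actor's location, each only if set.
; The actor destroys itself when the particle system finishes, or after a short delay if no effect is assigned.
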(event `SpawnBlast Efects`
  (bind _blastefects (`self.BlastEfects`)
    (:`then`
      (bind _returnvalue (`GameplayStatics.SpawnEmitterAttached` _blastefects (`self.DefaultSceneRoot`)))
      (add `ParticleSystemComponent.OnSystemFinished` _returnvalue (delegate `SystemFinished`)))
    (:`else`
      (`KismetSystemLibrary.Delay` 1.0)
      (`self.K2_DestroyActor`))))

(event `SystemFinished`
  (params (PSystem :type "ParticleSystemComponent Object Reference"))
  (`self.K2_DestroyActor`))

(event `Play Blast Sounds`
  (bind _blast_sound (`self.Blast Sound`)
    (:`then`
      (`GameplayStatics.PlaySoundAtLocation` _blast_sound (`self.K2_GetActorLocation`) (struct) 1.0 1.0 0.0 null null null null))
    (:`else`)))

(event `self.Trigger`
  (`parent.Trigger`)
  (`self.SpawnBlast Efects`)
  (`self.Play Blast Sounds`))

(fn `UserConstructionScript`
  (`parent.UserConstructionScript`))