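; Enemy character Blueprint for a katana-wielding AI that draws its sword on BeginPlay and exposes attack, sheathe, patrol route and movement speed functions.
; Montage notifies time the katana's spawn and attachment to the hand socket when drawing, and its destruction when sheathing.
; Event dispatchers report when draw, sheathe and attack montages end, with attack also reporting on interruption.
; SetMovementSpeed maps a movement state to max walk speed.
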(event `self.ReceiveBeginPlay`
  (`self.WildKatana`))

(event `Attack`
  (`|PlayMontage` (`self.Mesh`) "/Game/Wapons/KATANA/Animations/Montages/StableSwordOutwardSlash_Montage.StableSwordOutwardSlash_Montage"
    (:`OnCompleted`
      _)
    (:`OnInterrupted`
      _))
  (`self.OnAttackEnd`))

(event `WildKatana`
  (bind _notifyname (`|PlayMontage` (`self.Mesh`) "/Game/Wapons/KATANA/Animations/Montages/WithdrawingSword_UE_Montage.WithdrawingSword_UE_Montage")
    (:`OnCompleted`
      (`self.OnWildKatana`))
    (:`OnNotifyBegin`
      (switch `name` _notifyname
        (:`Desembainar`
          (bind _returnvalue (`|SpawnActorFromClass` "/Game/Wapons/KATANA/Blueprints/BP_Katana.BP_Katana_C" (`self.GetTransform`) "Undefined" "MultiplyWithRoot" null null))
          (bind _output_get (set `self.SwordActor` _returnvalue))
          (`self.K2_AttachToComponent` _output_get (`self.Mesh`) "hand_Sword_r_Socket" "SnapToTarget" "SnapToTarget" "SnapToTarget" true)
          (set `self.IsWiledingKatana?` true))))))

(event `SheatSword`
  (bind _notifyname (`|PlayMontage` (`self.Mesh`) "/Game/Wapons/KATANA/Animations/Montages/SheathingSword_UE_Montage.SheathingSword_UE_Montage")
    (:`OnCompleted`
      (`self.OnShietKatana`))
    (:`OnNotifyBegin`
      (switch `name` _notifyname
        (:`DropSword`
          (`self.K2_DestroyActor` (`self.SwordActor`))
          (set `self.IsWiledingKatana?` false))))))

(fn `GetPatrolRoute`
  (returns (PatrolRuote :type "/Game/Damage_System/Enemy/AI/BP_PatrolRoute Object Reference"))
  (return (`self.PatrolRoute`)))

(fn `SetMovementSpeed`
  (params (Speed :type "/Game/Damage_System/Enemy/AI/Enums/E_MovementSpeed Enum" :default "NewEnumerator0"))
  (returns (SpeedValue :type "Float (double-precision)"))
  (bind _output_get (set `CharacterMovementComponent.MaxWalkSpeed` (select `/Game/Damage_System/Enemy/AI/Enums/E_MovementSpeed` Speed :`NewEnumerator1` 100.0 :`NewEnumerator2` 300.0 :`NewEnumerator3` 500.0 :!type "Float (single-precision)") (`self.CharacterMovement`)))
  (return _output_get))

(fn `UserConstructionScript`)