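; Ranged enemy character that spawns with a rifle attached to its hand socket and shoots at its attack target.
; It extends a parent enemy class, overriding movement speed tiers and the ideal attack and defend range.
; Attacks play a firing montage whose notify has BPCAttacks trace a blockable bullet from weapon to target, then end on completion or interruption.
; Incoming damage passes to BPCDamageSystem, and the AttackStart override always returns false.
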(event `self.ReceiveBeginPlay`
  (`parent.ReceiveBeginPlay`)
  (`self.EquipWapon`))

(event `/Game/Characters/AI_Enemy/AI/BPI_EnemyAI.EquipWapon`
  (bind _returnvalue (`|SpawnActorFromClass` "/Game/Wapons/Blueprints/BP_Wapon_Rifle.BP_Wapon_Rifle_C" (`KismetMathLibrary.MakeTransform` (0.0 0.0 0.0)) "Undefined" "MultiplyWithRoot" null null))
  (bind _output_get (set `self.WaponActor` _returnvalue))
  (`self.K2_AttachToComponent` _output_get (`self.Mesh`) "hand_r_Rifle_Socket" "SnapToTarget" "SnapToTarget" "SnapToTarget" true)
  (set `self.IsWiledingWapon` true)
  (`self.OnWaponEquip`))

(event `/Game/Characters/AI_Enemy/AI/BPI_EnemyAI.Attack`
  (params (AttackTarget :type "Actor Object Reference"))
  (`parent.Attack` AttackTarget)
  (bind _notifyname (`|PlayMontage` (`self.Mesh`) "/Game/Characters/AI_Enemy/AI/Animations/EnemygoDsitancia/DisparoRifle_UE_Montage.DisparoRifle_UE_Montage")
    (:`OnCompleted`
      (`self.AttackEnd` AttackTarget :!label _label))
    (:`OnInterrupted`
      (goto _label))
    (:`OnNotifyBegin`
      (switch `name` _notifyname
        (:`Fire`
          (`/Game/Attacks/BPC_Attacks.FireBullet` (`self.BPC_Attacks`) (`self.K2_GetActorLocation` (`self.WaponActor`)) (`self.K2_GetActorLocation` AttackTarget) (make `/Game/Damage_System/S_DamageInfo` 15.0 "NewEnumerator2" "NewEnumerator0" false true)))))))

(fn `AttackStart`
  (params (AttackTarget :type "Actor Object Reference") (TokkenNeeded :type Integer))
  (returns (Success :type Boolean))
  (return false))

(fn `GetIdealRange`
  (returns (AttackRadius :type "Float (double-precision)") (DefendRadius :type "Float (double-precision)"))
  (return 600.0 600.0))

(fn `SetMovementSpeed`
  (params (Speed :type "/Game/Characters/AI_Enemy/AI/Enums/E_MovementSpeed Enum" :default "NewEnumerator0"))
  (returns (SpeedValue :type "Float (double-precision)"))
  (bind _output_get (set `CharacterMovementComponent.MaxWalkSpeed` (select `/Game/Characters/AI_Enemy/AI/Enums/E_MovementSpeed` Speed :`NewEnumerator1` 200.0 :`NewEnumerator2` 300.0 :`NewEnumerator3` 500.0 :!type "Float (single-precision)") (`self.CharacterMovement`)))
  (return _output_get))

(fn `TakeDamage`
  (params (DamageInfo :type "/Game/Damage_System/S_DamageInfo Structure") (`Damage Causer` :type "Actor Object Reference"))
  (returns (`Was Damagabele` :type Boolean))
  (if (`.CanBeBlocked_13_C02A7C97424F2BB0E6255E9B49109D8A` (break `/Game/Damage_System/S_DamageInfo` DamageInfo))
    _
    (else
      _))
  (bind _was_damaged (`/Game/Damage_System/BPC_DamageSystem.TakeDamage` (`self.BPC_DamageSystem`) DamageInfo `Damage Causer`))
  (return _was_damaged))

(fn `UserConstructionScript`
  (`parent.UserConstructionScript`))