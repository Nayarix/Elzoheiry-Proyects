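; Sword-wielding melee enemy character that supplies the attack, weapon and range behavior for its AI.
; Attack events (long-range jump, short slash, spin, ground smash) package damage info and a montage for the BPCAttacks component to execute.
; Equip and unequip montages use notifies to spawn and socket-attach or destroy the katana, then signal completion.
; GetIdealRange supplies fixed attack and defend radii, while SetMovementSpeed only returns zero.
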(event `self.ReceiveBeginPlay`
  (`parent.ReceiveBeginPlay`))

(event `LongRangueAttack`
  (params (AttackTarget :type "Actor Object Reference"))
  (`/Game/Attacks/BPC_Attacks.LongRangueMeleeAttack` (`self.BPC_Attacks`) (make `/Game/Damage_System/S_AttackInfo` AttackTarget (make `/Game/Damage_System/S_DamageInfo` 15.0 "NewEnumerator1" "NewEnumerator0" false true true) "/Game/Characters/AI_Enemy/AI/Animations/EnemigoMelle/AM_SwordJumpAttack.AM_SwordJumpAttack")))

(event `/Game/Characters/AI_Enemy/AI/BPI_EnemyAI.EquipWapon`
  (bind _notifyname (`|PlayMontage` (`self.Mesh`) "/Game/Wapons/KATANA/Animations/Montages/WithdrawingSword_UE_Montage.WithdrawingSword_UE_Montage")
    (:`OnCompleted`
      (`self.OnWaponEquip`))
    (:`OnNotifyBegin`
      (switch `name` _notifyname
        (:`Desembainar`
          (bind _returnvalue (`|SpawnActorFromClass` "/Game/Wapons/Blueprints/BP_Wapon_Katana.BP_Wapon_Katana_C" (`self.GetTransform`) "Undefined" "MultiplyWithRoot" null null))
          (bind _output_get (set `self.WaponActor` _returnvalue))
          (`self.K2_AttachToComponent` _output_get (`self.Mesh`) "hand_Sword_r_Socket" "SnapToTarget" "SnapToTarget" "SnapToTarget" true)
          (set `self.IsWiledingWapon` true))))))

(event `ShortRamgueAttack`
  (params (AttackTarget :type "Actor Object Reference"))
  (`/Game/Attacks/BPC_Attacks.PrimaryMeleeAttack` (`self.BPC_Attacks`) (make `/Game/Damage_System/S_AttackInfo` AttackTarget (make `/Game/Damage_System/S_DamageInfo` 10.0 "NewEnumerator1" "NewEnumerator0" false true true) "/Game/Wapons/KATANA/Animations/Montages/StableSwordOutwardSlash_Montage.StableSwordOutwardSlash_Montage") 20.0 200.0))

(event `/Game/Characters/AI_Enemy/AI/BPI_EnemyAI.UnequipWapon`
  (bind _notifyname (`|PlayMontage` (`self.Mesh`) "/Game/Wapons/KATANA/Animations/Montages/SheathingSword_UE_Montage.SheathingSword_UE_Montage")
    (:`OnCompleted`
      (`self.OnWaponUnequip`))
    (:`OnNotifyBegin`
      (switch `name` _notifyname
        (:`DropSword`
          (`self.K2_DestroyActor` (`self.WaponActor`))
          (set `self.IsWiledingWapon` false))))))

(event `SpiningAttack`
  (params (`AttackTarget ` :type "Actor Object Reference"))
  (`/Game/Attacks/BPC_Attacks.SpiningMeleeAttack` (`self.BPC_Attacks`) (make `/Game/Damage_System/S_AttackInfo` `AttackTarget ` (make `/Game/Damage_System/S_DamageInfo` 5.0 "NewEnumerator1" "NewEnumerator0" false true) "/Game/Characters/AI_Enemy/AI/Animations/EnemigoMelle/AM_SwordSpiningAttack.AM_SwordSpiningAttack")))

(event `GroundSmashAttack`
  (params (AttackTarget :type "Actor Object Reference"))
  (`/Game/Attacks/BPC_Attacks.GroundSmash` (`self.BPC_Attacks`) (make `/Game/Damage_System/S_AttackInfo` AttackTarget (make `/Game/Damage_System/S_DamageInfo` 30.0 "NewEnumerator3") "/Game/Characters/AI_Enemy/AI/Animations/EnemigoMelle/AM_MeleeGroundSmash.AM_MeleeGroundSmash") 300.0))

(fn `CalculateFutureActorLocation`
  (params (Actor :type "Actor Object Reference") (Time :type "Float (double-precision)" :default 1.0))
  (returns (Location :type "Vector Structure"))
  (return (+ (`self.K2_GetActorLocation` Actor) (* (* (`self.GetVelocity` Actor) (1.0 1.0 0.0)) Time))))

(fn `GetIdealRange`
  (returns (AttackRadius :type "Float (double-precision)") (DefendRadius :type "Float (double-precision)"))
  (return 200.0 400.0))

(fn `SetMovementSpeed`
  (params (Speed :type "/Game/Characters/AI_Enemy/AI/Enums/E_MovementSpeed Enum" :default "NewEnumerator0"))
  (returns (SpeedValue :type "Float (double-precision)"))
  (return 0.0))

(fn `UserConstructionScript`
  (`parent.UserConstructionScript`)
  (set `self.MeshRotationBeforeSpin` (`SceneComponent.RelativeRotation` (`self.Mesh`))))