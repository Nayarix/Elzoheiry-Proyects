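; Enemy mage character with basic spell, barrage and ground smash attacks run through BPCAttacks, plus teleport and self-heal abilities that signal completion via dispatchers.
; Teleport is faked: the mage turns invisible, ignores pawn collision and flies at high speed via AIMoveTo with particle effects.
; Healing plays a montage and spawns a line-trace-placed AOE that heals only the mage.
; It also supplies movement speeds and ideal ranges, and forwards damage to BPCDamageSystem.
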(event `BarrageAttack`
  (params (AttackTarget :type "Actor Object Reference"))
  (`/Game/Attacks/BPC_Attacks.BarrageMageAttack` (`self.BPC_Attacks`) (make `/Game/Damage_System/S_AttackInfo` AttackTarget (make `/Game/Damage_System/S_DamageInfo` 5.0 "NewEnumerator2") "/Game/Characters/Enemy/Mage/Animations/AM_MageCastBarrage.AM_MageCastBarrage")))

(event `BasicAttack`
  (params (AttackTarget :type "Actor Object Reference"))
  (`/Game/Attacks/BPC_Attacks.BasicMageSpell` (`self.BPC_Attacks`) (make `/Game/Damage_System/S_AttackInfo` AttackTarget (make `/Game/Damage_System/S_DamageInfo` 20.0 "NewEnumerator2") "/Game/Characters/Enemy/Mage/Animations/AM_MontageFireballMage.AM_MontageFireballMage")))

(event `GroundSmashAttack`
  (params (AttackTarget :type "Actor Object Reference"))
  (`/Game/Attacks/BPC_Attacks.GroundSmash` (`self.BPC_Attacks`) (make `/Game/Damage_System/S_AttackInfo` AttackTarget (make `/Game/Damage_System/S_DamageInfo` 30.0 "NewEnumerator3") "/Game/Characters/Enemy/Mage/Animations/AM_SmashGroundAttackMAGE.AM_SmashGroundAttackMAGE") 300.0))

(event `Teleport`
  (params (Location :type "Vector Structure"))
  (bind _charactermovement (`self.CharacterMovement`))
  (if (not (`self.IsTeleporting`))
    (set `self.IsTeleporting` true)
    (`CharacterMovementComponent.SetMovementMode` _charactermovement "MOVE_Flying" 0)
    (set `CharacterMovementComponent.MaxFlySpeed` 5000.0 _charactermovement)
    (set `CharacterMovementComponent.MaxAcceleration` 99999.0 _charactermovement)
    (`SceneComponent.SetVisibility` (`self.Mesh`) false true)
    (`PrimitiveComponent.SetCollisionResponseToChannel` (`self.CapsuleComponent`) "ECC_Pawn" "ECR_Ignore")
    (bind _returnvalue (`GameplayStatics.SpawnEmitterAttached` "/Game/InfinityBladeEffects/Effects/FX_Monsters/FX_Monster_Ausar/P_AU_Heal_01.P_AU_Heal_01" (`self.Mesh`) "Spine1"))
    (set `self.TeleportBodyEfect` _returnvalue)
    (bind _returnvalue_2 (`GameplayStatics.SpawnEmitterAttached` "/Game/InfinityBladeEffects/Effects/FX_Mobile/ICE/combat/P_AOE_Ice_CircleAttack.P_AOE_Ice_CircleAttack" (`self.Mesh`) "Spine1"))
    (set `self.TeleportTrialEfect` _returnvalue_2)
    (`self.StopAnimMontage` null)
    (`|AIMoveTo` self Location null 15.0
      (:`OnSuccess`
        _)
      (:`OnFail`
        _))
    (`self.TeleportEnd`)
    (else
      (`KismetSystemLibrary.DelayUntilNextTick`)
      (`self.OnTeleportEnd`))))

(event `TeleportEnd`
  (bind _charactermovement (`self.CharacterMovement`))
  (`MovementComponent.StopMovementImmediately` _charactermovement)
  (`CharacterMovementComponent.SetMovementMode` _charactermovement "MOVE_Walking" 0)
  (set `CharacterMovementComponent.MaxAcceleration` 1500.0 _charactermovement)
  (`SceneComponent.SetVisibility` (`self.Mesh`) true true)
  (`PrimitiveComponent.SetCollisionResponseToChannel` (`self.CapsuleComponent`) "ECC_Pawn" "ECR_Block")
  (`self.OnTeleportEnd`)
  (`KismetSystemLibrary.Delay` 0.5)
  (set `self.IsTeleporting` false)
  (`|ExecutionSequence`
    (:`then_0`
      (bind _teleportbodyefect (`self.TeleportBodyEfect`)
        (:`then`
          (`ActorComponent.K2_DestroyComponent` _teleportbodyefect))
        (:`else`)))
    (:`then_1`
      (bind _teleporttrialefect (`self.TeleportTrialEfect`)
        (:`then`
          (`ActorComponent.K2_DestroyComponent` _teleporttrialefect))
        (:`else`)))))

(event `HealOvertime`
  (bind _returnvalue (`self.K2_GetActorLocation`))
  (`|PlayMontage` (`self.Mesh`) "/Game/Characters/Enemy/Mage/Animations/AM_MageHeal.AM_MageHeal"
    (:`then`
      (bind (_outhit _returnvalue_2) (`KismetSystemLibrary.LineTraceSingle` _returnvalue (* _returnvalue (0.0 0.0 -1000.0)) "TraceTypeQuery1"))
      (if _returnvalue_2
        (bind _returnvalue_3 (`|SpawnActorFromClass` "/Game/AOE/BP_AOE_Overtime_Cura.BP_AOE_Overtime_Cura_C" (`KismetMathLibrary.MakeTransform` (`.Location` (`GameplayStatics.BreakHitResult` _outhit))) "Undefined" "MultiplyWithRoot" null 1.0 5.0 false false true null))
        (bind _output_get (set `self.HealAOE` _returnvalue_3))
        (add `/Game/AOE/BP_AOE_Base.OnAOE_OverlapActor` _output_get (delegate `OnHealTick`))
        (else
          (`self.StopAnimMontage` null))))
    (:`OnCompleted`
      (`self.HealOvertineEnded` :!label _label))
    (:`OnInterrupted`
      (goto _label))))

(event `OnHealTick`
  (params (Actor :type "Actor Object Reference"))
  (if (== Actor self)
    (`self.Heal` (* (`/Game/Damage_System/BPC_DamageSystem.MaxHealth` (`self.BPC_DamageSystem`)) 0.05))))

(event `HealOvertineEnded`
  (`self.OnHealOvetimeEnd`)
  (bind _healaoe (`self.HealAOE`)
    (:`then`
      (`self.K2_DestroyActor` _healaoe))
    (:`else`)))

(fn `GetIdealRange`
  (returns (AttackRadius :type "Float (double-precision)") (DefendRadius :type "Float (double-precision)"))
  (return 500.0 700.0))

(fn `SetMovementSpeed`
  (params (Speed :type "/Game/Characters/AI_Enemy/AI/Enums/E_MovementSpeed Enum" :default "NewEnumerator0"))
  (returns (SpeedValue :type "Float (double-precision)"))
  (return (select `/Game/Characters/AI_Enemy/AI/Enums/E_MovementSpeed` Speed :`NewEnumerator1` 150.0 :`NewEnumerator2` 250.0 :`NewEnumerator3` 400.0)))

(fn `TakeDamage`
  (params (DamageInfo :type "/Game/Damage_System/S_DamageInfo Structure") (`Damage Causer` :type "Actor Object Reference"))
  (returns (`Was Damagabele` :type Boolean))
  (bind _was_damaged (`/Game/Damage_System/BPC_DamageSystem.TakeDamage` (`self.BPC_DamageSystem`) DamageInfo `Damage Causer`))
  (return _was_damaged))

(fn `UserConstructionScript`
  (`parent.UserConstructionScript`))