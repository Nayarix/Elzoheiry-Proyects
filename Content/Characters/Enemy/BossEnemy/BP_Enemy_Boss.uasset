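; Boss enemy character, a child enemy Blueprint with a large health pool, an axe weapon and its own health bar widget.
; Creates the health bar on BeginPlay and refreshes it from the damage system component after the parent TakeDamage runs.
; Equip spawns the axe on a hand socket and unequip destroys it, each notifying a tick later.
; SetMovementSpeed maps movement states to boss-specific walk speeds.
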(event `self.ReceiveBeginPlay`
  (bind _bpc_damagesystem (`self.BPC_DamageSystem`))
  (`parent.ReceiveBeginPlay`)
  (bind _returnvalue (`|CreateWidget` "/Game/Widgets/W_BossHealtBar.W_BossHealtBar_C"))
  (bind _output_get (set `self.BossHealthBarWidgetReference` _returnvalue))
  (`/Game/Widgets/W_BossHealtBar.UpdateHealtPercentage` _output_get (`/Game/Damage_System/BPC_DamageSystem.MaxHealth` _bpc_damagesystem) (`/Game/Damage_System/BPC_DamageSystem.Health` _bpc_damagesystem)))

(event `/Game/Characters/AI_Enemy/AI/BPI_EnemyAI.EquipWapon`
  (bind _returnvalue (`|SpawnActorFromClass` "/Game/Wapons/Blueprints/BP_Wapon_Axx.BP_Wapon_Axx_C" (`KismetMathLibrary.MakeTransform` (0.0 0.0 0.0)) "Undefined" "MultiplyWithRoot" null null))
  (bind _output_get (set `self.WaponActor` _returnvalue))
  (`self.K2_AttachToComponent` _output_get (`self.Mesh`) "hand_r_Axx_Socket" "SnapToTarget" "SnapToTarget" "SnapToTarget" true)
  (set `self.IsWiledingWapon` true)
  (`KismetSystemLibrary.DelayUntilNextTick`)
  (`self.OnWaponEquip`))

(event `/Game/Characters/AI_Enemy/AI/BPI_EnemyAI.UnequipWapon`
  (`self.K2_DestroyActor` (`self.WaponActor`))
  (set `self.IsWiledingWapon` false)
  (`KismetSystemLibrary.DelayUntilNextTick`)
  (`self.OnWaponUnequip`))

(fn `SetMovementSpeed`
  (params (Speed :type "/Game/Characters/AI_Enemy/AI/Enums/E_MovementSpeed Enum" :default "NewEnumerator0"))
  (returns (SpeedValue :type "Float (double-precision)"))
  (bind _output_get (set `CharacterMovementComponent.MaxWalkSpeed` (select `/Game/Characters/AI_Enemy/AI/Enums/E_MovementSpeed` Speed :`NewEnumerator1` 100.0 :`NewEnumerator2` 200.0 :`NewEnumerator3` 350.0 :!type "Float (single-precision)") (`self.CharacterMovement`)))
  (return _output_get))

(fn `TakeDamage`
  (params (DamageInfo :type "/Game/Damage_System/S_DamageInfo Structure") (`Damage Causer` :type "Actor Object Reference"))
  (returns (`Was Damagabele` :type Boolean))
  (bind _bpc_damagesystem (`self.BPC_DamageSystem`))
  (bind _was_damagabele (`parent.TakeDamage` DamageInfo `Damage Causer`))
  (`/Game/Widgets/W_BossHealtBar.UpdateHealtPercentage` (`self.BossHealthBarWidgetReference`) (`/Game/Damage_System/BPC_DamageSystem.MaxHealth` _bpc_damagesystem) (`/Game/Damage_System/BPC_DamageSystem.Health` _bpc_damagesystem))
  (return _was_damagabele))

(fn `UserConstructionScript`
  (bind _bpc_damagesystem (`self.BPC_DamageSystem`))
  (`parent.UserConstructionScript`)
  (bind _output_get (set `/Game/Damage_System/BPC_DamageSystem.MaxHealth` 700.0 _bpc_damagesystem))
  (set `/Game/Damage_System/BPC_DamageSystem.Health` _output_get _bpc_damagesystem))