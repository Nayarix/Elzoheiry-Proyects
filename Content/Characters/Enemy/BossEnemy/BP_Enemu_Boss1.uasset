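; Axe-wielding boss enemy character with a boss health bar, a set of attacks, and teleport and invincible floating-platform abilities.
; Attacks either delegate to BPCAttacks or play montages whose notifies trigger traces, a homing axe throw, or a targeted AOE with damage callbacks.
; Teleport is a hidden, high-speed flying AI move with pawn collision ignored.
; Equip, float and teleport fire completion events, and TakeDamage refreshes the health bar.
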(event `self.ReceiveBeginPlay`
  (bind _bpc_damagesystem (`self.BPC_DamageSystem`))
  (`parent.ReceiveBeginPlay`)
  ;[1 1 1] HealtBar
  (bind _returnvalue (`|CreateWidget` "/Game/Widgets/W_BossHealtBar.W_BossHealtBar_C"))
  (bind _output_get (set `self.BossHealthBarWidgetReference` _returnvalue))
  (`/Game/Widgets/W_BossHealtBar.UpdateHealtPercentage` _output_get (`/Game/Damage_System/BPC_DamageSystem.MaxHealth` _bpc_damagesystem) (`/Game/Damage_System/BPC_DamageSystem.Health` _bpc_damagesystem)))

(event `/Game/Characters/AI_Enemy/AI/BPI_EnemyAI.EquipWapon`
  ;[1 1 1] Equip Onequip Wapon
  (bind _returnvalue (`|SpawnActorFromClass` "/Game/Wapons/Blueprints/BP_Wapon_Axx.BP_Wapon_Axx_C" (`KismetMathLibrary.MakeTransform` (0.0 0.0 0.0)) "Undefined" "MultiplyWithRoot" null null))
  (bind _output_get (set `self.WaponActor` _returnvalue))
  (`self.K2_AttachToComponent` _output_get (`self.Mesh`) "hand_r_Axx_Socket" "SnapToTarget" "SnapToTarget" "SnapToTarget" true)
  (set `self.IsWiledingWapon` true)
  (`KismetSystemLibrary.DelayUntilNextTick`)
  (`self.OnWaponEquip`))

(event `/Game/Characters/AI_Enemy/AI/BPI_EnemyAI.UnequipWapon`
  ;[1 1 1] Equip Onequip Wapon
  (`self.K2_DestroyActor` (`self.WaponActor`))
  (set `self.IsWiledingWapon` false)
  (`KismetSystemLibrary.DelayUntilNextTick`)
  (`self.OnWaponUnequip`))

(event `AttackCombo1`
  (params (AttackTarget :type "Actor Object Reference"))
  ;[1 1 1] Attacks
  (`/Game/Attacks/BPC_Attacks.PrimaryMeleeAttack` (`self.BPC_Attacks`) (make `/Game/Damage_System/S_AttackInfo` AttackTarget (make `/Game/Damage_System/S_DamageInfo` 20.0 "NewEnumerator1" "NewEnumerator1" false true true) "/Game/Characters/Enemy/BossEnemy/Animations/comboacha_UE_Montage.comboacha_UE_Montage") 40.0 220.0))

(event `AttackCombo2`
  (params (AttackTarget :type "Actor Object Reference"))
  (bind _bpc_attacks (`self.BPC_Attacks`))
  ;[1 1 1] Attacks
  (`self.Attack` AttackTarget)
  (bind _notifyname (`|PlayMontage` (`self.Mesh`) "/Game/Characters/Enemy/BossEnemy/Animations/comboacha2_UE_Montage.comboacha2_UE_Montage")
    (:`OnCompleted`
      (`/Game/Characters/AI_Enemy/AI/BPI_EnemyAI.AttackEnd` AttackTarget :!label _label))
    (:`OnInterrupted`
      (goto _label))
    (:`OnNotifyBegin`
      (switch `name` _notifyname
        (:`Slash`
          (`/Game/Attacks/BPC_Attacks.SphereTraceDamage` _bpc_attacks (make `/Game/Damage_System/S_DamageInfo` 15.0 "NewEnumerator1" "NewEnumerator1" false true true) 40.0 220.0))
        (:`AOESlash`
          (`/Game/Attacks/BPC_Attacks.AOEDamage` _bpc_attacks 300.0 (make `/Game/Damage_System/S_DamageInfo` 20.0 "NewEnumerator3" "NewEnumerator1" false false false true)))))))

(event `ThrowAxe`
  (params (AttackTarget :type "Actor Object Reference"))
  ;[1 1 1] Attacks
  (`/Game/Characters/AI_Enemy/AI/BPI_EnemyAI.Attack` AttackTarget)
  (bind _notifyname (`|PlayMontage` (`self.Mesh`) "/Game/Characters/Enemy/BossEnemy/Animations/lanzaracha_UE_Montage.lanzaracha_UE_Montage")
    (:`OnCompleted`
      (`SceneComponent.SetVisibility` (`/Game/Wapons/Blueprints/BP_Wapon_Base.Mesh` (`self.WaponActor`)) true false :!label _label_2)
      (`/Game/Characters/AI_Enemy/AI/BPI_EnemyAI.AttackEnd` AttackTarget))
    (:`OnInterrupted`
      (goto _label_2))
    (:`OnNotifyBegin`
      (switch `name` _notifyname
        (:`ThrowAxe`
          (`SceneComponent.SetVisibility` (`/Game/Wapons/Blueprints/BP_Wapon_Base.Mesh` (`self.WaponActor`)) false false)
          (bind _returnvalue (`|SpawnActorFromClass` "/Game/Proyectiles/BP_Proyectile_Spining_Axe.BP_Proyectile_Spining_Axe_C" (`KismetMathLibrary.MakeTransform` (`SceneComponent.GetSocketLocation` (`self.Mesh`) "hand_r")) "Undefined" "MultiplyWithRoot" null 4000.0 0.0 AttackTarget true self))
          (add `/Game/Proyectiles/BP_ProyectileBase.On Projectile Impact` _returnvalue (delegate `On Projectile Impact_Event`)))))))

(event `GroundSmash`
  (params (AttackTarget :type "Actor Object Reference"))
  ;[1 1 1] Attacks
  (`/Game/Attacks/BPC_Attacks.GroundSmash` (`self.BPC_Attacks`) (make `/Game/Damage_System/S_AttackInfo` AttackTarget (make `/Game/Damage_System/S_DamageInfo` 25.0 "NewEnumerator3" "NewEnumerator1" false false false true) "/Game/Characters/Enemy/BossEnemy/Animations/Area_Impact.Area_Impact") 1100.0))

(event `AOETrial`
  (params (AttackTarget :type "Actor Object Reference"))
  ;[1 1 1] Attacks
  (`self.Attack` AttackTarget)
  (bind _notifyname (`|PlayMontage` (`self.Mesh`) "/Game/Characters/Enemy/BossEnemy/Animations/Battlecry_UE_Montage.Battlecry_UE_Montage")
    (:`OnCompleted`
      (`/Game/Characters/AI_Enemy/AI/BPI_EnemyAI.AttackEnd` AttackTarget :!label _label_3))
    (:`OnInterrupted`
      (goto _label_3))
    (:`OnNotifyBegin`
      (switch `name` _notifyname
        (:`Strike`
          (bind _returnvalue (`|SpawnActorFromClass` "/Game/AOE/BP_AOE_Trueno.BP_AOE_Trueno_C" (`KismetMathLibrary.MakeTransform` (0.0 0.0 0.0)) "Undefined" "MultiplyWithRoot" null 3.0 AttackTarget false true false null))
          (add `/Game/AOE/BP_AOE_Base.OnAOE_OverlapActor` _returnvalue (delegate `OnAOE_OverlapActor_Event`)))))))

(event `QuikAttacks`
  (params (AttackTarget :type "Actor Object Reference"))
  ;[1 1 1] Attacks
  (`/Game/Attacks/BPC_Attacks.PrimaryMeleeAttack` (`self.BPC_Attacks`) (make `/Game/Damage_System/S_AttackInfo` AttackTarget (make `/Game/Damage_System/S_DamageInfo` 20.0 "NewEnumerator1" "NewEnumerator1" false true true) "/Game/Characters/Enemy/BossEnemy/Animations/GolpeBasicoBoss.GolpeBasicoBoss") 40.0 220.0))

(event `JumpAttack`
  (params (AttackTarget :type "Actor Object Reference"))
  ;[1 1 1] Attacks
  (`/Game/Attacks/BPC_Attacks.LongRangueMeleeAttack` (`self.BPC_Attacks`) (make `/Game/Damage_System/S_AttackInfo` AttackTarget (make `/Game/Damage_System/S_DamageInfo` 20.0 "NewEnumerator3" "NewEnumerator0" false false false true) "/Game/Characters/Enemy/BossEnemy/Animations/ataquesaltoacha_UE_Montage.ataquesaltoacha_UE_Montage")))

(event `On Projectile Impact_Event`
  (params (OtherActor :type "Actor Object Reference") (Hit :type "HitResult Structure"))
  ;[1 1 1] Attacks
  (message `/Game/Damage_System/BPI_Damagable.TakeDamage` OtherActor (make `/Game/Damage_System/S_DamageInfo` 20.0 "NewEnumerator2" "NewEnumerator1" false true) self))

(event `OnAOE_OverlapActor_Event`
  (params (Actor :type "Actor Object Reference"))
  ;[1 1 1] Attacks
  (bind _teamnumber (message `/Game/Damage_System/BPI_Damagable.GetTeamNumber` Actor))
  (if (!= _teamnumber (`self.Team Number`))
    (message `/Game/Damage_System/BPI_Damagable.TakeDamage` Actor (make `/Game/Damage_System/S_DamageInfo` 30.0 "NewEnumerator3" "NewEnumerator1") self)))

(event `StartFloat`
  (bind _returnvalue (`self.K2_GetActorLocation`))
  ;[1 1 1] Floating Pilar Hability
  (set `/Game/Damage_System/BPC_DamageSystem.IsInvencible` true (`self.BPC_DamageSystem`))
  (bind _outhit (`KismetSystemLibrary.LineTraceSingle` _returnvalue (* _returnvalue (1.0 1.0 -1000.0)) "TraceTypeQuery1"))
  (bind _returnvalue_2 (`|SpawnActorFromClass` "/Game/Props/BP_Plataform.BP_Plataform_C" (`KismetMathLibrary.MakeTransform` (`.Location` (`GameplayStatics.BreakHitResult` _outhit))) "Undefined" "MultiplyWithRoot" null null))
  (bind _output_get (set `self.FloatingPlataformREF` _returnvalue_2))
  (add `/Game/Props/BP_Plataform.OnFloatTimelineFinished` _returnvalue_2 (delegate `OnFloatTimelineFinished_Event`))
  (add `/Game/Props/BP_Plataform.OnFloatTimelineFinished` _output_get (delegate `OnFloatTimelineFinished_Event`)))

(event `Teleport`
  (params (Location :type "Vector Structure") (AttackTarget :type "Actor Object Reference"))
  (bind _charactermovement (`self.CharacterMovement`))
  ;[1 1 1] Teleport
  (if (not (`self.IsTeleporting`))
    (set `self.IsTeleporting` true)
    (`CharacterMovementComponent.SetMovementMode` _charactermovement "MOVE_Flying" 0)
    (set `CharacterMovementComponent.MaxFlySpeed` 5000.0 _charactermovement)
    (set `CharacterMovementComponent.MaxAcceleration` 99999.0 _charactermovement)
    (`SceneComponent.SetVisibility` (`self.Mesh`) false true)
    (`PrimitiveComponent.SetCollisionResponseToChannel` (`self.CapsuleComponent`) "ECC_Pawn" "ECR_Ignore")
    (bind _returnvalue (`GameplayStatics.SpawnEmitterAttached` "/Game/InfinityBladeEffects/Effects/FX_Mobile/ICE/combat/P_AOE_Ice_CircleAttack.P_AOE_Ice_CircleAttack" (`self.Mesh`) "spine_01"))
    (set `self.TeleportTrialEfect` _returnvalue)
    (`self.StopAnimMontage` null)
    (`|AIMoveTo` self Location AttackTarget 150.0
      (:`OnSuccess`
        _)
      (:`OnFail`
        _))
    (`self.TeleportEnd`)
    (else
      (`KismetSystemLibrary.DelayUntilNextTick`)
      (`self.OnTeleportEnd`))))

(event `OnFloatTimelineFinished_Event`
  ;[1 1 1] Floating Pilar Hability
  (remove `/Game/Props/BP_Plataform.OnFloatTimelineFinished` (stale `StartFloat` _output_get) (delegate `OnFloatTimelineFinished_Event`))
  (`self.OnFloatHeightReached`))

(event `StopFloat`
  ;[1 1 1] Floating Pilar Hability
  (bind _floatingplataformref (`self.FloatingPlataformREF`)
    (:`then`
      (`/Game/Props/BP_Plataform.StopFloting` _floatingplataformref)
      (add `/Game/Props/BP_Plataform.OnFloatTimelineFinished` _floatingplataformref (delegate `OnFloatTimelineFinished_Event_0`)))
    (:`else`
      (`KismetSystemLibrary.DelayUntilNextTick`)
      (set `/Game/Damage_System/BPC_DamageSystem.IsInvencible` false (`self.BPC_DamageSystem`) :!label _label_4)
      (`self.OnFloatEnded`))))

(event `OnFloatTimelineFinished_Event_0`
  ;[1 1 1] Floating Pilar Hability
  (remove `/Game/Props/BP_Plataform.OnFloatTimelineFinished` (stale `StopFloat` _floatingplataformref) (delegate `OnFloatTimelineFinished_Event_0`))
  (`self.K2_DestroyActor` (stale `StopFloat` _floatingplataformref))
  (goto _label_4))

(event `TeleportEnd`
  (bind _charactermovement (`self.CharacterMovement`))
  ;[1 1 1] Teleport
  (`MovementComponent.StopMovementImmediately` _charactermovement)
  (`CharacterMovementComponent.SetMovementMode` _charactermovement "MOVE_Walking" 0)
  (set `CharacterMovementComponent.MaxAcceleration` 1500.0 _charactermovement)
  (`SceneComponent.SetVisibility` (`self.Mesh`) true true)
  (`PrimitiveComponent.SetCollisionResponseToChannel` (`self.CapsuleComponent`) "ECC_Pawn" "ECR_Block")
  (`self.OnTeleportEnd`)
  (`KismetSystemLibrary.Delay` 0.5)
  (set `self.IsTeleporting` false)
  (bind _teleporttrialefect (`self.TeleportTrialEfect`)
    (:`then`
      (`ActorComponent.K2_DestroyComponent` _teleporttrialefect))
    (:`else`)))

(fn `SetMovementSpeed`
  (params (Speed :type "/Game/Characters/AI_Enemy/AI/Enums/E_MovementSpeed Enum" :default "NewEnumerator0"))
  (returns (SpeedValue :type "Float (double-precision)"))
  (bind _output_get (set `CharacterMovementComponent.MaxWalkSpeed` (select `/Game/Characters/AI_Enemy/AI/Enums/E_MovementSpeed` Speed :`NewEnumerator1` 100.0 :`NewEnumerator2` 200.0 :`NewEnumerator3` 350.0 :!type "Float (single-precision)") (`self.CharacterMovement`)))
  (return _output_get))

(fn `TakeDamage`
  (params (DamageInfo :type "/Game/Damage_System/S_DamageInfo Structure") (`Damage Causer` :type "Actor Object Reference"))
  (returns (`Was Damagabele` :type Boolean))
  (bind _bpc_damagesystem (`self.BPC_DamageSystem`))
  (bind _was_damagabele (`parent.TakeDamage` DamageInfo `Damage Causer`))
  (`/Game/Widgets/W_BossHealtBar.UpdateHealtPercentage` (`self.BossHealthBarWidgetReference`) (`/Game/Damage_System/BPC_DamageSystem.MaxHealth` _bpc_damagesystem) (`/Game/Damage_System/BPC_DamageSystem.Health` _bpc_damagesystem))
  (return _was_damagabele))

(fn `UserConstructionScript`
  (bind _bpc_damagesystem (`self.BPC_DamageSystem`))
  (`parent.UserConstructionScript`)
  (bind _output_get (set `/Game/Damage_System/BPC_DamageSystem.MaxHealth` 700.0 _bpc_damagesystem))
  (set `/Game/Damage_System/BPC_DamageSystem.Health` _output_get _bpc_damagesystem))