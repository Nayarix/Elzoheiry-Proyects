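; Base projectile actor that flies toward an optional Target and reports what it hits.
; The construction script applies speed and gravity to ProjectileMovement and enables homing on the Target's root component when IsHoming is set.
; BeginPlay aims the velocity at the Target and makes the collision box ignore the instigator, or the owner as fallback.
; A box hit calls OnProjectileImpact, spawns the impact effect and sound, then destroys the projectile.
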(event `self.ReceiveBeginPlay`
  (bind _returnvalue (`self.GetInstigator`))
  ;[1 1 1] Begin Play
  (`self.Rotate to target`)
  (`PrimitiveComponent.IgnoreActorWhenMoving` (`self.Box Collision`) (select `bool` (`KismetSystemLibrary.IsValid` _returnvalue) :`false` (`self.GetOwner`) :`true` _returnvalue :!type "Actor Object Reference") true))

(event `Rotate to target`
  ;[1 1 1] Rotate to target
  (`self.Target`
    (:`then`
      (set `MovementComponent.Velocity` (* (`KismetMathLibrary.GetDirectionUnitVector` (`self.K2_GetActorLocation`) (`self.K2_GetActorLocation` (`self.Target`))) (`self.Speed`)) (`self.ProjectileMovement`)))
    (:`else`)))

(event `ImpactEfect`
  (params (Location :type "Vector Structure"))
  ;[1 1 1] Impact Efect
  (bind _impact_efect (`self.Impact Efect`)
    (:`then`
      (`GameplayStatics.SpawnEmitterAtLocation` _impact_efect Location))
    (:`else`)))

(event `Play Impact Sound`
  (params (Location :type "Vector Structure"))
  ;[1 1 1] Sound
  (bind _impact_sound (`self.Impact Sound`)
    (:`then`
      (`GameplayStatics.PlaySoundAtLocation` _impact_sound Location (struct) 1.0 1.0 0.0 null null null null))
    (:`else`)))

(event `self.Box Collision.OnComponentHit`
  (params (HitComponent :type "PrimitiveComponent Object Reference") (OtherActor :type "Actor Object Reference") (OtherComp :type "PrimitiveComponent Object Reference") (NormalImpulse :type "Vector Structure") (Hit :type "HitResult Structure (by ref)"))
  (bind (_bblockinghit _binitialoverlap _time _distance _location _impactpoint) (`GameplayStatics.BreakHitResult` Hit))
  (`self.On Projectile Impact` OtherActor Hit)
  (`self.ImpactEfect` _impactpoint)
  (`self.Play Impact Sound` _impactpoint)
  (`self.K2_DestroyActor`))

(fn `UserConstructionScript`
  (bind _projectilemovement (`self.ProjectileMovement`))
  (bind _speed (`self.Speed`))
  (set `ProjectileMovementComponent.InitialSpeed` _speed _projectilemovement)
  (set `ProjectileMovementComponent.MaxSpeed` _speed _projectilemovement)
  (set `ProjectileMovementComponent.ProjectileGravityScale` (`self.Gravity`) _projectilemovement)
  (`self.Target`
    (:`then`
      (if (`self.IsHoming`)
        (set `ProjectileMovementComponent.bIsHomingProjectile` true _projectilemovement)
        (set `ProjectileMovementComponent.HomingTargetComponent` (`Actor.RootComponent` (`self.Target`)) _projectilemovement)))
    (:`else`)))